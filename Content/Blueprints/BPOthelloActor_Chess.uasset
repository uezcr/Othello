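; Othello chess piece actor that animates its own spawning, flipping and removal on the board.
; A spawn timeline starts at BeginPlay and drives the mesh's height; SpawnTimeLine can play it backward, which destroys the actor when finished.
; ReverseTimeLine plays a second timeline in either direction, moving the mesh vertically while rolling it to flip the piece.
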(event EventBeginPlay
  (Components|Timeline|PlayfromStart (Variables|Default|GetTimeLine_Spawn)))

(event Collision|EventActorBeginOverlap
  (params (OtherActor :type Actor%20Object%20Reference)))

(event EventTick
  (params (DeltaSeconds :type Float%20%28single-precision%29)))

(event EventReverseTimeLine
  (params (IsForward :type Boolean))
  (bind _timeline_reverse (Variables|Default|GetTimeLine_Reverse))
  (if IsForward
    (Components|Timeline|PlayfromStart _timeline_reverse)
    (else
      (Components|Timeline|ReversefromEnd _timeline_reverse))))

(event EventSpawnTimeLine
  (params (IsForward :type Boolean))
  (bind _timeline_spawn (Variables|Default|GetTimeLine_Spawn))
  (if IsForward
    (Components|Timeline|PlayfromStart _timeline_spawn)
    (else
      (Components|Timeline|ReversefromEnd _timeline_spawn))))

(fn ConstructionScript)